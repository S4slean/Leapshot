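; BP_Ball is a physics ball that players can catch and launch.
; A catch radius overlap passes the ball's reference to BP_Player unless it is attached, and removes it when the player leaves.
; Events toggle the sphere's physics and collision, and Launch applies a velocity-change impulse.
; Reactivation restores Pawn blocking after a short delay, while deactivation ignores pawns.
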(event OnComponentBeginOverlap(CatchRadius)
  (params (OverlappedComponent :type Primitive%20Component%20Object%20Reference) (OtherActor :type Actor%20Object%20Reference) (OtherComp :type Primitive%20Component%20Object%20Reference) (OtherBodyIndex :type Integer) (bFromSweep :type Boolean) (SweepResult :type Hit%20Result%20Structure%20%28by%20ref%29))
  (bind (_asbp_player _bsuccess) (Utilities|Casting|CastToBP_Player OtherActor))
  (if (not (Variables|Default|GetbAttached))
    (if _bsuccess
      (Default|GetBallReference _asbp_player self))))

(event OnComponentEndOverlap(CatchRadius)
  (params (OverlappedComponent :type Primitive%20Component%20Object%20Reference) (OtherActor :type Actor%20Object%20Reference) (OtherComp :type Primitive%20Component%20Object%20Reference) (OtherBodyIndex :type Integer))
  (bind (_asbp_player _bsuccess) (Utilities|Casting|CastToBP_Player OtherActor))
  (if _bsuccess
    (Default|DeleteBallReference _asbp_player self)))

(event Custom|Activate%20Physics
  (bind _sphere (Variables|Default|GetSphere))
  (Physics|SetSimulatePhysics (Variables|Default|GetSphere) true)
  (Collision|SetCollisionEnabled _sphere "QueryAndPhysics")
  (Utilities|FlowControl|Delay 0.1)
  (Collision|SetCollisionResponsetoChannel _sphere "ECC_Pawn" "ECR_Block"))

(event Custom|Disable%20Physics
  (bind _sphere (Variables|Default|GetSphere))
  (Collision|SetCollisionResponsetoChannel (Variables|Default|GetSphere) "ECC_Pawn" "ECR_Ignore")
  (Physics|SetSimulatePhysics _sphere false)
  (Collision|SetCollisionEnabled _sphere "NoCollision"))

(event Custom|Launch
  (params (Impulse :type Vector))
  (Physics|AddImpulse (Variables|Default|GetSphere) Impulse "None" true))

(event Input|ActionEvents|InputActionPass/Intercept
  (params (Key :type Key%20Structure :default "None")))

(fn ConstructionScript)