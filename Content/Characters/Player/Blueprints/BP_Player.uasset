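; BP_Player is the player character Blueprint, turning input into movement, jumping and camera look.
; Move axes add movement input along the camera's forward and right vectors, with only forward input forced.
; An IsJumping flag gates Jump on press and clears on release.
; Mouse and stick look axes feed controller yaw and pitch through separate sensitivity variables, with no delta-time scaling.
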(event Input|ActionEvents|InputActionJump
  (params (Key :type Key%20Structure :default "None"))
  (:Pressed
    (if (not (Variables|Default|GetbIsJumping))
      (Variables|Default|SetbIsJumping true)
      (Character|Jump)))
  (:Released
    (Variables|Default|SetbIsJumping false)
    (Character|StopJumping)))

(event Input|AxisEvents|InputAxisMoveForward
  (params (AxisValue :type Float%20%28single-precision%29))
  ;[1 1 1] Movement
  (bind _output_get (Variables|Input|SetForward AxisValue))
  (Pawn|Input|AddMovementInput (Math|Vector|GetForwardVector (Variables|Default|GetCamera)) _output_get true))

(event Input|AxisEvents|InputAxisMoveRight
  (params (AxisValue :type Float%20%28single-precision%29))
  ;[1 1 1] Movement
  (bind _output_get (Variables|Input|SetRight AxisValue))
  (Pawn|Input|AddMovementInput (Math|Vector|GetRightVector (Variables|Default|GetCamera)) _output_get false))

(event Input|AxisEvents|InputAxisTurn
  (params (AxisValue :type Float%20%28single-precision%29))
  ;[1 1 1] Camera
  (Pawn|Input|AddControllerYawInput (* AxisValue (Variables|Camera|GetmouseXSensitivity))))

(event Input|AxisEvents|InputAxisTurnRate
  (params (AxisValue :type Float%20%28single-precision%29))
  ;[1 1 1] Camera
  (Pawn|Input|AddControllerYawInput (* AxisValue (Variables|Camera|GetCamStickXSensitivity))))

(event Input|AxisEvents|InputAxisLookUp
  (params (AxisValue :type Float%20%28single-precision%29))
  ;[1 1 1] Camera
  (Pawn|Input|AddControllerPitchInput (* AxisValue (Variables|Camera|GetmouseYSensitivty))))

(event Input|AxisEvents|InputAxisLookUpRate
  (params (AxisValue :type Float%20%28single-precision%29))
  ;[1 1 1] Camera
  (Pawn|Input|AddControllerPitchInput (* AxisValue (Variables|Camera|GetCamStickYSensitivity))))

(fn ConstructionScript)